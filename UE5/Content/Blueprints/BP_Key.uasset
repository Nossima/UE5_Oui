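; BP_Key is a pickup key that unlocks portals requiring it.
; On overlap with a BP_ThirdPersonCharacter or BP_Character, it searches all BP_Portal actors in the level.
; Any portal whose NeededItem is this key has its NeedItem flag cleared, then the key destroys itself.
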(event `self.ReceiveActorBeginOverlap`
  (params (OtherActor :type "Actor Object Reference"))
  (bind _returnvalue (`GameplayStatics.GetObjectClass` OtherActor))
  (if (or (`KismetMathLibrary.ClassIsChildOf` _returnvalue "/Game/ThirdPerson/Blueprints/BP_ThirdPersonCharacter.BP_ThirdPersonCharacter_C") (`KismetMathLibrary.ClassIsChildOf` _returnvalue "/Game/Blueprints/BP_Character.BP_Character_C"))
    (bind _outactors (`GameplayStatics.GetAllActorsOfClass` "/Game/Blueprints/BP_Portal.BP_Portal_C"))
    (for _array_element _outactors
      (if (== (`/Game/Blueprints/BP_Portal.NeedItem` _array_element) true)
        (if (== (`/Game/Blueprints/BP_Portal.NeededItem` _array_element) self)
          (set `/Game/Blueprints/BP_Portal.NeedItem` false _array_element))))
    (`self.K2_DestroyActor`)))

(fn `UserConstructionScript`)