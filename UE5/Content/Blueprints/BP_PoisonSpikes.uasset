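; BP_PoisonSpikes is a spike trap that rises and poisons the Greystone player character.
; Overlapping the Collision component snaps the actor up by Distance with a swept move, then lowers it after a delay.
; A separate Box overlap calls GetPoisoned on the player.
; IsUp blocks re-triggering while raised, and DidPoison limits poisoning to once until the spikes next lower.
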(event OnComponentBeginOverlap(Collision)
  (params (OverlappedComponent :type Primitive%20Component%20Object%20Reference) (OtherActor :type Actor%20Object%20Reference) (OtherComp :type Primitive%20Component%20Object%20Reference) (OtherBodyIndex :type Integer) (bFromSweep :type Boolean) (SweepResult :type Hit%20Result%20Structure%20%28by%20ref%29))
  (Utilities|Casting|CastToBP_GreystonePlayerCharacter OtherActor)
  (CallFunction|SpikesUp))

(event OnComponentBeginOverlap(Box)
  (params (OverlappedComponent :type Primitive%20Component%20Object%20Reference) (OtherActor :type Actor%20Object%20Reference) (OtherComp :type Primitive%20Component%20Object%20Reference) (OtherBodyIndex :type Integer) (bFromSweep :type Boolean) (SweepResult :type Hit%20Result%20Structure%20%28by%20ref%29))
  (if (not (Variables|Default|GetDidPoison))
    (bind _asbp_greystone_player_character (Utilities|Casting|CastToBP_GreystonePlayerCharacter OtherActor))
    (Default|GetPoisoned _asbp_greystone_player_character 1)
    (Variables|Default|SetDidPoison true)))

(event Custom|SpikesUp
  (bind _self self)
  (bind _returnvalue (Transformation|GetActorLocation _self))
  (bind (_x _y _z) (Class|KismetMathLibrary|BreakVector3f _returnvalue))
  (if (not (Variables|Default|GetIsUp))
    (Transformation|SetActorLocation (Math|Vector|MakeVector _x _y (+ _z (Variables|Default|GetDistance))) true false)
    (Variables|Default|SetIsUp true)
    (Utilities|FlowControl|Delay 3.0)
    (CallFunction|SpikesDown)))

(event Custom|SpikesDown
  (bind _self self)
  (bind _returnvalue (Transformation|GetActorLocation _self))
  (bind (_x _y _z) (Class|KismetMathLibrary|BreakVector3f _returnvalue))
  (Transformation|SetActorLocation (Math|Vector|MakeVector _x _y (- _z (Variables|Default|GetDistance))) true false)
  (Variables|Default|SetIsUp false)
  (Variables|Default|SetDidPoison false))

(event EventBeginPlay)

(event Collision|EventActorBeginOverlap
  (params (OtherActor :type Actor%20Object%20Reference)))

(event EventTick
  (params (DeltaSeconds :type Float%20%28single-precision%29)))

(fn ConstructionScript)